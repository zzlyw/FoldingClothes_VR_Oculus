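; Image capture actor that connects to a server by IP, sends a picture and projects two axis and two finger points into the scene.
; TakePicture parses the IP string, connects and sends the first picture.
; Tick rescales the points from a fixed resolution to the viewport with aspect-ratio offsets, then deprojects and line-traces against Pawns to position four marker actors.
; When new data is flagged, it fires a dispatcher and notifies the receive thread.
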(event EventBeginPlay
  (Variables|/Script/Engine.PlayerController|SetbShowMouseCursor (Game|GetPlayerController 0) true)
  (Variables|Default|SetPoses (Utilities|Array|MakeArray (Variables|Default|GetPos1) (Variables|Default|GetPos2) (Variables|Default|GetPos3) (Variables|Default|GetPos4)))
  (bind _returnvalue (UserInterface|CreateWidget "/Game/Blueprints/MyUI_BP.MyUI_BP_C"))
  (bind _output_get (Variables|Default|SetMyUI _returnvalue))
  (UserInterface|Viewport|AddtoViewport _output_get 0)
  (Variables|Default|SetIPs (Utilities|Array|MakeArray (Variables|Default|GetIP0) (Variables|Default|GetIP1) (Variables|Default|GetIP2) (Variables|Default|GetIP3))))

(event EventTick
  (params (DeltaSeconds :type Float%20%28single-precision%29))
  (bind _returnvalue (Viewport|GetViewportSize))
  (Utilities|FlowControl|Sequence
    (:then_0
      (Variables|Default|SetWHRatio (/ (Math|Conversions|ToFloat(Integer) (Variables|Default|GetFixWidth)) (Math|Conversions|ToFloat(Integer) (Variables|Default|GetFixHeight))))
      (Variables|Default|SetWHRatio_current (/ (.x _returnvalue) (.y _returnvalue)))
      (if (>= (Variables|Default|GetWHRatio_current) (Variables|Default|GetWHRatio))
        (Variables|Default|SetAdd_X_axis true)
        (Variables|Default|SetoffsetPixels (* (/ (- (Variables|Default|GetWHRatio_current) (Variables|Default|GetWHRatio)) 2.0) (.y (Viewport|GetViewportSize))))
        (else
          (Variables|Default|SetAdd_X_axis false)
          (Variables|Default|SetoffsetPixels (* (/ (- (/ 1.0 (Variables|Default|GetWHRatio_current)) (/ 1.0 (Variables|Default|GetWHRatio))) 2.0) (.x (Viewport|GetViewportSize)))))))
    (:then_1
      (Variables|Default|SetData (Utilities|Array|MakeArray (Math|Vector2D|MakeVector2D (Variables|Default|GetaxisPoint1_x) (Variables|Default|GetaxisPoint1_y)) (Math|Vector2D|MakeVector2D (Variables|Default|GetaxisPoint2_x) (Variables|Default|GetaxisPoint2_y)) (Math|Vector2D|MakeVector2D (Variables|Default|GetfingerPoint1_x) (Variables|Default|GetfingerPoint1_y)) (Math|Vector2D|MakeVector2D (Variables|Default|GetfingerPoint2_x) (Variables|Default|GetfingerPoint2_y))))
      (for _index (range 0 3)
        (Utilities|Array|SetArrayElem (Variables|Default|GetData) _index (Math|Vector2D|MakeVector2D (+ (* (.x (Utilities|Array|Get(acopy) (Variables|Default|GetData) _index)) (select (Variables|Default|GetAdd_X_axis) (/ (.y (Viewport|GetViewportSize)) (Math|Conversions|ToFloat(Integer) (Variables|Default|GetFixHeight))) (/ (.x (Viewport|GetViewportSize)) (Math|Conversions|ToFloat(Integer) (Variables|Default|GetFixWidth))))) (select (Variables|Default|GetAdd_X_axis) (Variables|Default|GetoffsetPixels) 0.0)) (+ (* (.y (Utilities|Array|Get(acopy) (Variables|Default|GetData) _index)) (select (Variables|Default|GetAdd_X_axis) (/ (.y (Viewport|GetViewportSize)) (Math|Conversions|ToFloat(Integer) (Variables|Default|GetFixHeight))) (/ (.x (Viewport|GetViewportSize)) (Math|Conversions|ToFloat(Integer) (Variables|Default|GetFixWidth))))) (select (Variables|Default|GetAdd_X_axis) 0.0 (Variables|Default|GetoffsetPixels))))))
      (for _index_2 (range 0 3)
        (bind _outhit (Collision|LineTraceForObjects (.WorldLocation (Class|PlayerController|DeprojectScreenPositiontoWorld (Game|GetPlayerController 0) (.X (Math|Vector2D|BreakVector2D (Utilities|Array|Get(acopy) (Variables|Default|GetData) _index_2))) (.Y (Math|Vector2D|BreakVector2D (Utilities|Array|Get(acopy) (Variables|Default|GetData) _index_2))))) (+ (.WorldLocation (Class|PlayerController|DeprojectScreenPositiontoWorld (Game|GetPlayerController 0) (.X (Math|Vector2D|BreakVector2D (Utilities|Array|Get(acopy) (Variables|Default|GetData) _index_2))) (.Y (Math|Vector2D|BreakVector2D (Utilities|Array|Get(acopy) (Variables|Default|GetData) _index_2))))) (* (.WorldDirection (Class|PlayerController|DeprojectScreenPositiontoWorld (Game|GetPlayerController 0) (.X (Math|Vector2D|BreakVector2D (Utilities|Array|Get(acopy) (Variables|Default|GetData) _index_2))) (.Y (Math|Vector2D|BreakVector2D (Utilities|Array|Get(acopy) (Variables|Default|GetData) _index_2))))) 1e+03)) (Utilities|Array|MakeArray "ObjectTypeQuery3") false 0 "None"))
        (Transformation|SetActorLocation (Utilities|Array|Get(acopy) (Variables|Default|GetPoses) _index_2) (.Location (Collision|BreakHitResult _outhit)) false false)))
    (:then_2
      (if (Variables|Default|GetIsNewDataComing)
        (Default|CallEDImageCaptureActor)
        (Class|ImageCaptureActor|SetIsNewDataCominginReceiveThread)
        (Variables|Default|SetIsNewDataComing true)))))

(event Input|ActionEvents|InputActionTakePicture
  (params (Key :type Key%20Structure))
  (bind _ipaddress (Variables|Default|GetIPAddress))
  (:Pressed
    (Development|PrintString _ipaddress)
    (bind _output_get (Variables|Default|Setstrs_IP (Utilities|String|ParseIntoArray _ipaddress ".")))
    (if (>= (Utilities|Array|Length _output_get) 4)
      (Variables|Default|SetIP0 (Math|Conversions|ToByte(Integer) (Math|Conversions|ToInteger(Byte) (Utilities|Array|Get(acopy) (Variables|Default|Getstrs_IP)))))
      (Variables|Default|SetIP1 (Math|Conversions|ToByte(Integer) (Math|Conversions|ToInteger(Byte) (Utilities|Array|Get(acopy) (Variables|Default|Getstrs_IP) 1))))
      (Variables|Default|SetIP2 (Math|Conversions|ToByte(Integer) (Math|Conversions|ToInteger(Byte) (Utilities|Array|Get(acopy) (Variables|Default|Getstrs_IP) 2))))
      (Variables|Default|SetIP3 (Math|Conversions|ToByte(Integer) (Math|Conversions|ToInteger(Byte) (Utilities|Array|Get(acopy) (Variables|Default|Getstrs_IP) 3))))
      (Development|PrintString "Connecting Server ..." true true "(R=0.000000,G=0.660000,B=1.000000,A=1.000000)" 3e+01)
      (Class|ImageCaptureActor|ConnectServer)
      (Development|PrintString "Server connected!" true true "(R=0.000000,G=0.660000,B=1.000000,A=1.000000)" 3e+01)
      (Class|ImageCaptureActor|TakePictureandSend)
      (Development|PrintString "First picture sent!" true true "(R=0.000000,G=0.660000,B=1.000000,A=1.000000)" 3e+01)
      (else
        (Development|PrintString "IP Address Format Error!" true true "(R=0.000000,G=0.660000,B=1.000000,A=1.000000)" 1e+01)))))

(fn ConstructionScript)